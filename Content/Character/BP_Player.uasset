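; BP_Player is the player character, with Enhanced Input controls for looking, walking, jumping, sprinting and shooting.
; BeginPlay adds the IMC_POE mapping context; movement follows control yaw, and sprint swaps the walk speed while held.
; Every tick, velocity and a CanJump check choose an idle, walk or sprint camera shake.
; Primary shoot spawns BP_Projectile at SceneSpawnPoint, aimed along the camera's rotation.
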(event Custom|CameraShake
  (bind _returnvalue (Transformation|GetVelocity))
  (bind _returnvalue_2 (Game|GetPlayerCharacter 0))
  (bind _returnvalue_3 (Math|Vector|VectorLength _returnvalue))
  (bind _playerstate (Variables|/Script/Engine.Pawn|GetPlayerState _returnvalue_2))
  (bind _returnvalue_4 (Game|GetPlayerController _playerstate))
  ;[0.09531 0.000304 0.15 0.502] Camera Shake for Idle, Walk, and Sprint Movement
  (if (and (> _returnvalue_3 0.0) (Character|CanJump))
    (if (< _returnvalue_3 3e+02)
      (Game|Feedback|ClientStartCameraShake _returnvalue_4 "/Game/Character/CameraShake/WalkCamShake.WalkCamShake_C" 1.0 "CameraLocal" "0, 0, 0")
      (else
        (Game|Feedback|ClientStartCameraShake _returnvalue_4 "/Game/Character/CameraShake/SprintCamShake.SprintCamShake_C" 1.0 "CameraLocal" "0, 0, 0")))
    (else
      (Game|Feedback|ClientStartCameraShake _returnvalue_4 "/Game/Character/CameraShake/IdleCamShake.IdleCamShake_C" 1.0 "CameraLocal" "0, 0, 0"))))

(event Input|EnhancedActionEvents|EnhancedInputActionIA_MouseLook_POE
  (params (ActionValue :type Vector%202D%20Structure) (ElapsedSeconds :type Float%20%28double-precision%29) (TriggeredSeconds :type Float%20%28double-precision%29) (InputAction :type Input%20Action%20Object%20Reference :default "/Game/Input/IA_MouseLook_POE.IA_MouseLook_POE"))
  ;[0.09531 0.000304 0.15 0.502] Mouse Camera Movement
  (Pawn|Input|AddControllerYawInput (.x ActionValue))
  (Pawn|Input|AddControllerPitchInput (* (.y ActionValue) -1.0)))

(event Input|EnhancedActionEvents|EnhancedInputActionIA_Walk_POE
  (params (ActionValue :type Vector%202D%20Structure) (ElapsedSeconds :type Float%20%28double-precision%29) (TriggeredSeconds :type Float%20%28double-precision%29) (InputAction :type Input%20Action%20Object%20Reference :default "/Game/Input/IA_Walk_POE.IA_Walk_POE"))
  (bind _returnvalue (Pawn|GetControlRotation :!class /Script/Engine.Pawn))
  ;[0.09531 0.000304 0.15 0.502] WASD Controls
  (Pawn|Input|AddMovementInput (Math|Vector|GetRightVector (Math|Rotator|MakeRotator (.roll _returnvalue) 0.0 (.yaw _returnvalue))) (.x ActionValue) false)
  (Pawn|Input|AddMovementInput (Math|Vector|GetForwardVector (Math|Rotator|MakeRotator 0.0 0.0 (.yaw (Pawn|GetControlRotation :!class /Script/Engine.Pawn)))) (.y ActionValue) false))

(event Input|EnhancedActionEvents|EnhancedInputActionIA_Jump_POE
  (params (ActionValue :type Boolean) (ElapsedSeconds :type Float%20%28double-precision%29) (TriggeredSeconds :type Float%20%28double-precision%29) (InputAction :type Input%20Action%20Object%20Reference :default "/Game/Input/IA_Jump_POE.IA_Jump_POE"))
  ;[0.09531 0.000304 0.15 0.502] Jump Action
  (:Triggered
    (Character|Jump))
  (:Completed
    (Character|StopJumping)))

(event Input|EnhancedActionEvents|EnhancedInputActionIA_Sprint_POE
  (params (ActionValue :type Boolean) (ElapsedSeconds :type Float%20%28double-precision%29) (TriggeredSeconds :type Float%20%28double-precision%29) (InputAction :type Input%20Action%20Object%20Reference :default "/Game/Input/IA_Sprint_POE.IA_Sprint_POE"))
  (bind _charactermovement (Variables|Character|GetCharacterMovement))
  ;[0.09531 0.000304 0.15 0.502] Sprint Action
  (:Started
    (Variables|/Script/Engine.CharacterMovementComponent|SetMaxWalkSpeed _charactermovement 1.2e+03))
  (:Completed
    (Variables|/Script/Engine.CharacterMovementComponent|SetMaxWalkSpeed _charactermovement 6e+02)))

(event Input|EnhancedActionEvents|EnhancedInputActionIA_PrimaryShoot
  (params (ActionValue :type Boolean) (ElapsedSeconds :type Float%20%28double-precision%29) (TriggeredSeconds :type Float%20%28double-precision%29) (InputAction :type Input%20Action%20Object%20Reference :default "/Game/Input/IA_PrimaryShoot.IA_PrimaryShoot"))
  ;[0.09531 0.000304 0.15 0.502] Shoot Bullets
  (:Started
    (Game|SpawnActorfromClass "/Game/Character/BP_Projectile.BP_Projectile_C" (Math|Transform|MakeTransform (Transformation|GetWorldLocation (Variables|Default|GetScene%20%28spawnPoint%29)) (Transformation|GetWorldRotation (Variables|Default|GetCamera_Player))) "Undefined" "MultiplyWithRoot" 0 0)))

(event EventBeginPlay
  ;[0.09531 0.000304 0.15 0.502] BeginPlay - the Start() function in Unity
  (bind _asplayer_controller (Utilities|Casting|CastToPlayerController (Pawn|GetController)))
  (Utilities|IsValid (PlayerController|LocalPlayerSubsystems|GetEnhancedInputLocalPlayerSubsystem _asplayer_controller)
    (:Is%20Valid
      (Input|AddMappingContext (PlayerController|LocalPlayerSubsystems|GetEnhancedInputLocalPlayerSubsystem _asplayer_controller) "/Game/Input/IMC_POE.IMC_POE" 0 "(bIgnoreAllPressedKeysUntilRelease=True,bForceImmediately=False,bNotifyUserSettings=False)"))))

(event Collision|EventActorBeginOverlap
  (params (OtherActor :type Actor%20Object%20Reference)))

(event EventTick
  (params (DeltaSeconds :type Float%20%28single-precision%29))
  ;[0 0.15 0.04381 0.5] EVENT TICK [the Update() in Unity]
  (CallFunction|CameraShake))

(fn ConstructionScript)